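; BP_ShelfArea is a shelf drop zone in a platypus warehouse game that accepts boxes and awards score.
; The construction script hides its Box component as a placeholder.
; When a BP_NBox overlaps the Trigger, it is destroyed and the placeholder becomes visible, making the box appear shelved.
; It then casts player 0's character to the warehouse platypus to increase and update the score.
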(event `self.Trigger.OnComponentBeginOverlap`
  (params (OverlappedComponent :type "PrimitiveComponent Object Reference") (OtherActor :type "Actor Object Reference") (OtherComp :type "PrimitiveComponent Object Reference") (OtherBodyIndex :type Integer) (bFromSweep :type Boolean) (SweepResult :type "HitResult Structure (by ref)"))
  (bind _asbp_nbox (cast `/Game/BP_NBox` OtherActor))
  (`self.K2_DestroyActor` _asbp_nbox)
  (`SceneComponent.SetVisibility` (`self.Box`) true false)
  (bind _asbp_third_person_character_platypus_warehouse (cast `/Game/BP_ThirdPersonCharacterPlatypusWarehouse` (`GameplayStatics.GetPlayerCharacter` 0)))
  (`/Game/BP_ThirdPersonCharacterPlatypusWarehouse.ScoreIncrease` _asbp_third_person_character_platypus_warehouse)
  (`/Game/BP_ThirdPersonCharacterPlatypusWarehouse.UpdateScore` _asbp_third_person_character_platypus_warehouse))

(fn `UserConstructionScript`
  (`SceneComponent.SetVisibility` (`self.Box`) false false))