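; BP_Hub is a level-transition trigger that banks the player's score and advances the day/night state.
; When a BP_Character overlaps the Trigger component, it adds the character's score to the BP_GameInstance total, flips IsDay and increments the Night counter on every pass.
; It then opens the TestEnvironment level by name, with the game instance holding that state across the load.
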(event `self.Trigger.OnComponentBeginOverlap`
  (params (OverlappedComponent :type "PrimitiveComponent Object Reference") (OtherActor :type "Actor Object Reference") (OtherComp :type "PrimitiveComponent Object Reference") (OtherBodyIndex :type Integer) (bFromSweep :type Boolean) (SweepResult :type "HitResult Structure (by ref)"))
  (bind _asbp_character (cast `/Game/Dylan/Blueprints/BP_Character` OtherActor))
  (`KismetSystemLibrary.PrintString` "Loading")
  (bind _asbp_game_instance (cast `/Game/Dylan/Blueprints/BP_GameInstance` (`GameplayStatics.GetGameInstance`)))
  (set `/Game/Dylan/Blueprints/BP_GameInstance.Score` (+ (`/Game/Dylan/Blueprints/BP_Character.Score` _asbp_character) (`/Game/Dylan/Blueprints/BP_GameInstance.Score` _asbp_game_instance)) _asbp_game_instance)
  (set `/Game/Dylan/Blueprints/BP_GameInstance.IsDay?` (not (`/Game/Dylan/Blueprints/BP_GameInstance.IsDay?` _asbp_game_instance)) _asbp_game_instance)
  (set `/Game/Dylan/Blueprints/BP_GameInstance.Night` (+ (`/Game/Dylan/Blueprints/BP_GameInstance.Night` _asbp_game_instance) 1) _asbp_game_instance)
  (`GameplayStatics.OpenLevel` "TestEnvironment"))

(fn `UserConstructionScript`)