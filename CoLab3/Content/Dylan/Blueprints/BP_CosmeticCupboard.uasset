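; BP_CosmeticCupboard is an interactable cupboard that opens a wardrobe UI.
; A trigger overlap shows a spotlight and prompt and enables Interact, which alternates open and close through a FlipFlop.
; Opening blends the view to the cupboard and swings both hinges on a timeline, then enters cinematic mode and shows WB_Wardrobe with the cursor.
; Closing removes these, blends to the "MainCam" actor and reverses the timeline, releasing cinematic mode when finished.
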(event `self.ReceiveBeginPlay`
  (`SceneComponent.SetHiddenInGame` (`self.SpotLight`) true false)
  (`SceneComponent.SetHiddenInGame` (`self.InteractText`) true false))

(event `self.Trigger.OnComponentBeginOverlap`
  (params (OverlappedComponent :type "PrimitiveComponent Object Reference") (OtherActor :type "Actor Object Reference") (OtherComp :type "PrimitiveComponent Object Reference") (OtherBodyIndex :type Integer) (bFromSweep :type Boolean) (SweepResult :type "HitResult Structure (by ref)"))
  (`SceneComponent.SetHiddenInGame` (`self.SpotLight`) false false)
  (`SceneComponent.SetHiddenInGame` (`self.InteractText`) false false)
  (set `self.Nearby?` true))

(event `self.Trigger.OnComponentEndOverlap`
  (params (OverlappedComponent :type "PrimitiveComponent Object Reference") (OtherActor :type "Actor Object Reference") (OtherComp :type "PrimitiveComponent Object Reference") (OtherBodyIndex :type Integer))
  (`SceneComponent.SetHiddenInGame` (`self.SpotLight`) true false)
  (`SceneComponent.SetHiddenInGame` (`self.InteractText`) true false)
  (set `self.Nearby?` false))

(event `/Game/Dylan/Blueprints/Interfaces/BPI_Interact.Interact`
  (bind _returnvalue (`GameplayStatics.GetPlayerController` 0))
  (if (`self.Nearby?`)
    (`/Engine/EditorBlueprintResources/StandardMacros.FlipFlop`
      (:`A`
        (`KismetSystemLibrary.PrintString` "OPEN!")
        (`PlayerController.SetViewTargetWithBlend` (`GameplayStatics.GetPlayerController` 0) self 1.0 "VTBlend_Linear" 0.0 false)
        (bind (_direction _open) (`Timeline|Open'` :!label _label)
          (:`Update`
            (bind _returnvalue_2 (`KismetMathLibrary.Lerp` 0.0 110.0 _open))
            (`SceneComponent.K2_SetRelativeRotation` (`self.Hinge1`) (`KismetMathLibrary.MakeRotator` 0.0 0.0 (* _returnvalue_2 -1.0)) false false)
            (`SceneComponent.K2_SetRelativeRotation` (`self.Hinge`) (`KismetMathLibrary.MakeRotator` 0.0 0.0 _returnvalue_2) false false))
          (:`Finished`
            (if (`|EnumEquality` _direction "Backward")
              (`PlayerController.SetCinematicMode` _returnvalue false true true true true)
              (else
                (`PlayerController.SetCinematicMode` _returnvalue true true true true true)
                (bind _returnvalue_3 (`|CreateWidget` "/Game/Dylan/UI/WB_Wardrobe.WB_Wardrobe_C"))
                (`UserWidget.AddToViewport` _returnvalue_3 0)
                (set `self.Widget` _returnvalue_3)
                (set `PlayerController.bShowMouseCursor` true (`GameplayStatics.GetPlayerController` 0)))))))
      (:`B`
        (`Widget.RemoveFromParent` (`self.Widget`))
        (set `PlayerController.bShowMouseCursor` false (`GameplayStatics.GetPlayerController` 0))
        (`KismetSystemLibrary.PrintString` "CLOSE!")
        (bind _outactors (`GameplayStatics.GetAllActorsWithTag` "MainCam"))
        (for _array_element _outactors
          (`PlayerController.SetViewTargetWithBlend` _returnvalue _array_element 1.0 "VTBlend_Linear" 0.0 false)
          (goto _label :!via `Reverse`))))))

(fn `UserConstructionScript`)