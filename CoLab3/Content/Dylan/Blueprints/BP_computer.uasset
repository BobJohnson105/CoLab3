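; BP_computer is an interactable in-world computer that shows a spotlight and text prompt while something overlaps its trigger.
; Interact toggles between blending the view to the computer in cinematic mode and returning to the MainCam-tagged camera, removing the screen widget.
; After the blend, it shows a day or night screen from the game instance, or a blank one if the landlord hasn't departed and Night isn't above zero.
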(event `self.ReceiveBeginPlay`
  (`SceneComponent.SetHiddenInGame` (`self.SpotLight`) true false)
  (`SceneComponent.SetHiddenInGame` (`self.TextRender`) true false))

(event `self.Trigger.OnComponentBeginOverlap`
  (params (OverlappedComponent :type "PrimitiveComponent Object Reference") (OtherActor :type "Actor Object Reference") (OtherComp :type "PrimitiveComponent Object Reference") (OtherBodyIndex :type Integer) (bFromSweep :type Boolean) (SweepResult :type "HitResult Structure (by ref)"))
  (`SceneComponent.SetHiddenInGame` (`self.SpotLight`) false false)
  (`SceneComponent.SetHiddenInGame` (`self.TextRender`) false false)
  (set `self.Nearby?` true))

(event `self.Trigger.OnComponentEndOverlap`
  (params (OverlappedComponent :type "PrimitiveComponent Object Reference") (OtherActor :type "Actor Object Reference") (OtherComp :type "PrimitiveComponent Object Reference") (OtherBodyIndex :type Integer))
  (`SceneComponent.SetHiddenInGame` (`self.SpotLight`) true false)
  (`SceneComponent.SetHiddenInGame` (`self.TextRender`) true false)
  (set `self.Nearby?` false))

(event `/Game/Dylan/Blueprints/Interfaces/BPI_Interact.Interact`
  (bind _returnvalue (`GameplayStatics.GetPlayerController` 0))
  (bind _returnvalue_2 (`GameplayStatics.GetPlayerController` 0))
  (if (`self.Nearby?`)
    (`/Engine/EditorBlueprintResources/StandardMacros.FlipFlop`
      (:`A`
        (`KismetSystemLibrary.PrintString` "PC ON!")
        (`PlayerController.SetViewTargetWithBlend` _returnvalue_2 self 1.0 "VTBlend_Linear" 0.0 false)
        (`PlayerController.SetCinematicMode` _returnvalue_2 true true true true true)
        (`KismetSystemLibrary.Delay` 1.0)
        (bind _outactors (`GameplayStatics.GetAllActorsWithTag` "Landlord"))
        (bind _asbp_landlord (cast `/Game/Dylan/Blueprints/BP_Landlord` (`|GetArrayItem` _outactors)))
        (bind _asbp_game_instance (cast `/Game/Dylan/Blueprints/BP_GameInstance` (`GameplayStatics.GetGameInstance`)))
        (if (`/Game/Dylan/Blueprints/BP_Landlord.Departed?` _asbp_landlord)
          (if (`/Game/Dylan/Blueprints/BP_GameInstance.IsDay?` _asbp_game_instance) :!label _label
            (bind _returnvalue_3 (`|CreateWidget` "/Game/Dylan/UI/WB_Computer_Day.WB_Computer_Day_C"))
            (`UserWidget.AddToViewport` _returnvalue_3 0)
            (set `self.Screen` _returnvalue_3)
            (else
              (bind _returnvalue_4 (`|CreateWidget` "/Game/Dylan/UI/WB_Computer_Night.WB_Computer_Night_C"))
              (`UserWidget.AddToViewport` _returnvalue_4 0)
              (set `self.Screen` _returnvalue_4)))
          (set `PlayerController.bShowMouseCursor` true (`GameplayStatics.GetPlayerController` 0))
          (elif (> (`/Game/Dylan/Blueprints/BP_GameInstance.Night` _asbp_game_instance) 0)
            (goto _label)
            (else
              (bind _returnvalue_5 (`|CreateWidget` "/Game/Dylan/UI/WB_ComputerBlank.WB_ComputerBlank_C"))
              (`UserWidget.AddToViewport` _returnvalue_5 0)
              (set `self.Screen` _returnvalue_5)))))
      (:`B`
        (`KismetSystemLibrary.PrintString` "PC OFF!")
        (bind _outactors_2 (`GameplayStatics.GetAllActorsWithTag` "MainCam"))
        (for _array_element _outactors_2
          (`PlayerController.SetViewTargetWithBlend` _returnvalue _array_element 1.0 "VTBlend_Linear" 0.0 false)
          (`PlayerController.SetCinematicMode` _returnvalue false true true true true)
          (`Widget.RemoveFromParent` (`self.Screen`))
          (set `PlayerController.bShowMouseCursor` false (`GameplayStatics.GetPlayerController` 0)))))))

(fn `UserConstructionScript`)