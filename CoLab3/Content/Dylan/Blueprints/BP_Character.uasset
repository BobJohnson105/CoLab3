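; Player character Blueprint that handles movement, interaction and the start of each day or night phase.
; Input moves and rotates the character and sphere-traces for BPI_Interact actors or components, while an overlap trigger tracks the current BPI_Dialogue component.
; Play reads BP_GameInstance, plays day/night transitions, shows the HUD and blends to MainCam.
; It then starts the landlord's arrival on night zero, or later shows win/lose screens by day and score.
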(event `EnhancedInput|/Game/Dylan/Inputs/IA_Interact`
  (params (ActionValue :type Boolean) (ElapsedSeconds :type "Float (double-precision)") (TriggeredSeconds :type "Float (double-precision)") (InputAction :type "InputAction Object Reference" :default "/Game/Dylan/Inputs/IA_Interact.IA_Interact"))
  (bind _capsulecomponent (`Character.CapsuleComponent` (`GameplayStatics.GetPlayerCharacter` 0)))
  (bind _returnvalue (`SceneComponent.K2_GetComponentLocation` _capsulecomponent))
  (:`Triggered`
    (bind _outhit (`KismetSystemLibrary.SphereTraceSingle` _returnvalue (+ _returnvalue (* (`SceneComponent.GetForwardVector` _capsulecomponent) 1000.0)) 60.0 "TraceTypeQuery1"))
    (bind (_bblockinghit _binitialoverlap _time _distance _location _impactpoint _normal _impactnormal _physmat _hitactor _hitcomponent) (`GameplayStatics.BreakHitResult` _outhit))
    (if (and (`KismetSystemLibrary.IsValid` _hitactor) (`KismetSystemLibrary.DoesImplementInterface` _hitactor "/Game/Dylan/Blueprints/Interfaces/BPI_Interact.BPI_Interact_C"))
      (message `/Game/Dylan/Blueprints/Interfaces/BPI_Interact.Interact` _hitactor)
      (elif (and (`KismetSystemLibrary.DoesImplementInterface` _hitcomponent "/Game/Dylan/Blueprints/Interfaces/BPI_Interact.BPI_Interact_C") (`KismetSystemLibrary.IsValid` _hitcomponent))
        (message `/Game/Dylan/Blueprints/Interfaces/BPI_Interact.Interact` _hitcomponent)
        (else
          (`KismetSystemLibrary.PrintString` "FailInteract!"))))))

(event `Play`
  (bind _asbp_game_instance (cast `/Game/Dylan/Blueprints/BP_GameInstance` (`GameplayStatics.GetGameInstance`)))
  (bind _output_get (set `self.Daytime?` (`/Game/Dylan/Blueprints/BP_GameInstance.IsDay?` _asbp_game_instance)))
  (if _output_get
    (bind _day (`/Game/Dylan/Blueprints/BP_GameInstance.Day` _asbp_game_instance))
    (set `self.Time` (`|FormatText` "Day {0}" (`|GenericToText` _day)))
    (else
      (bind _night (`/Game/Dylan/Blueprints/BP_GameInstance.Night` _asbp_game_instance))
      (set `self.Time` (`|FormatText` "Night {0}" (`|GenericToText` _night)))))
  (set `self.Score` (`/Game/Dylan/Blueprints/BP_GameInstance.Score` _asbp_game_instance))
  (if (== _night 0)
    (bind _returnvalue (`|CreateWidget` "/Game/Dylan/UI/WB_MainUI.WB_MainUI_C" :!label _label))
    (`UserWidget.AddToViewport` _returnvalue 0)
    (`/Game/Dylan/UI/WB_MainUI.UpdateScoreTime` _returnvalue (`self.Time`) (`self.Score`))
    (bind _outactors (`GameplayStatics.GetAllActorsWithTag` "MainCam"))
    (for _array_element _outactors
      (`PlayerController.SetViewTargetWithBlend` (`GameplayStatics.GetPlayerController` 0) _array_element 1.0 "VTBlend_Linear" 0.0 false)
      (`self.SetActorHiddenInGame` false)
      (bind _outactors_2 (`GameplayStatics.GetAllActorsWithTag` "Landlord"))
      (if (> _night 0)
        (if (>= _day 7)
          (if (>= (`self.Score`) 600.0)
            (bind _returnvalue_2 (`|CreateWidget` "/Game/Dylan/UI/WB_GameWin.WB_GameWin_C"))
            (`UserWidget.AddToViewport` _returnvalue_2 0)
            (else
              (bind _returnvalue_3 (`|CreateWidget` "/Game/Dylan/UI/WB_GameOver.WB_GameOver_C"))
              (`UserWidget.AddToViewport` _returnvalue_3 0))))
        (else
          (bind _asbp_landlord (cast `/Game/Dylan/Blueprints/BP_Landlord` (`|GetArrayItem` _outactors_2)))
          (`/Game/Dylan/Blueprints/BP_Landlord.Arrival` _asbp_landlord))))
    (else
      (bind _returnvalue_4 (`|CreateWidget` "/Game/Dylan/UI/WB_ChangeDay.WB_ChangeDay_C"))
      (`UserWidget.AddToViewport` _returnvalue_4 0)
      (if (`self.Daytime?`)
        (`|PlayAnimation2` _returnvalue_4 (`/Game/Dylan/UI/WB_ChangeDay.MoontoSun` _returnvalue_4)
          (:`then`
            _)
          (:`Finished`
            (`Widget.RemoveFromParent` _returnvalue_4 :!label _label_2)
            (goto _label)))
        (else
          (`|PlayAnimation2` _returnvalue_4 (`/Game/Dylan/UI/WB_ChangeDay.SuntoMoon` _returnvalue_4)
            (:`then`
              _)
            (:`Finished`
              (goto _label_2)))))
      (bind _returnvalue_5 (`GameplayStatics.SpawnSound2D` "/Game/Dylan/SFX/TransitionTheme.TransitionTheme" 1.0 1.0 0.0 null))
      (`KismetSystemLibrary.Delay` 26.0)
      (`AudioComponent.FadeOut` _returnvalue_5 10.0 0.0 "Linear"))))

(event `LevelStart`
  ; Test
  (bind _returnvalue (`|CreateWidget` "/Game/Dylan/UI/WB_MainUI.WB_MainUI_C"))
  (`UserWidget.AddToViewport` _returnvalue 0))

(event `EnhancedInput|/Game/Dylan/Inputs/IA_Movement`
  (params (ActionValue :type "Vector2D Structure") (ElapsedSeconds :type "Float (double-precision)") (TriggeredSeconds :type "Float (double-precision)") (InputAction :type "InputAction Object Reference" :default "/Game/Dylan/Inputs/IA_Movement.IA_Movement"))
  (bind _returnvalue (`KismetMathLibrary.Conv_Vector2DToVector` ActionValue))
  (:`Triggered`
    (`self.AddMovementInput` _returnvalue)
    (`self.K2_SetActorRotation` (`KismetMathLibrary.MakeRotationFromAxes` _returnvalue))))

(event `UpdateScore`
  ; Test
  (`/Game/Dylan/UI/WB_MainUI.UpdateScoreTime` (stale `LevelStart` _returnvalue) "" (`self.Score`)))

(event `self.DialogueTrigger.OnComponentBeginOverlap`
  (params (OverlappedComponent :type "PrimitiveComponent Object Reference") (OtherActor :type "Actor Object Reference") (OtherComp :type "PrimitiveComponent Object Reference") (OtherBodyIndex :type Integer) (bFromSweep :type Boolean) (SweepResult :type "HitResult Structure (by ref)"))
  (set `self.DialogueActor` (`|GetArrayItem` (`self.GetComponentsByInterface` OtherActor "/Game/Dylan/Blueprints/Interfaces/BPI_Dialogue.BPI_Dialogue_C"))))

(event `self.DialogueTrigger.OnComponentEndOverlap`
  (params (OverlappedComponent :type "PrimitiveComponent Object Reference") (OtherActor :type "Actor Object Reference") (OtherComp :type "PrimitiveComponent Object Reference") (OtherBodyIndex :type Integer))
  (`/Engine/EditorBlueprintResources/StandardMacros.IsValid` OtherActor
    (:`Is Valid`
      (set `self.DialogueActor` null))))

(fn `UserConstructionScript`)