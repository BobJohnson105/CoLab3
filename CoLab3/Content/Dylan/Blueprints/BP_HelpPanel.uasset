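; BP_HelpPanel is an interactable help panel that reveals a spotlight and help text while something overlaps its box.
; Both start hidden, and the overlap events also set a Nearby flag that gates Interact.
; Interact alternates between blending the view to the panel in cinematic mode and blending back to the MainCam-tagged actor with cinematic mode off, printing a debug string each time.
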(event `self.ReceiveBeginPlay`
  (`SceneComponent.SetHiddenInGame` (`self.SpotLight`) true false)
  (`SceneComponent.SetHiddenInGame` (`self.HelpText`) true false))

(event `self.Box.OnComponentBeginOverlap`
  (params (OverlappedComponent :type "PrimitiveComponent Object Reference") (OtherActor :type "Actor Object Reference") (OtherComp :type "PrimitiveComponent Object Reference") (OtherBodyIndex :type Integer) (bFromSweep :type Boolean) (SweepResult :type "HitResult Structure (by ref)"))
  (`SceneComponent.SetHiddenInGame` (`self.SpotLight`) false false)
  (`SceneComponent.SetHiddenInGame` (`self.HelpText`) false false)
  (set `self.Nearby?` true))

(event `self.Box.OnComponentEndOverlap`
  (params (OverlappedComponent :type "PrimitiveComponent Object Reference") (OtherActor :type "Actor Object Reference") (OtherComp :type "PrimitiveComponent Object Reference") (OtherBodyIndex :type Integer))
  (`SceneComponent.SetHiddenInGame` (`self.SpotLight`) true false)
  (`SceneComponent.SetHiddenInGame` (`self.HelpText`) true false)
  (set `self.Nearby?` false))

(event `/Game/Dylan/Blueprints/Interfaces/BPI_Interact.Interact`
  (bind _returnvalue (`GameplayStatics.GetPlayerController` 0))
  (if (`self.Nearby?`)
    (`/Engine/EditorBlueprintResources/StandardMacros.FlipFlop`
      (:`A`
        (`KismetSystemLibrary.PrintString` "HELP!")
        (`PlayerController.SetViewTargetWithBlend` (`GameplayStatics.GetPlayerController` 0) self 1.0 "VTBlend_Linear" 0.0 false)
        (`PlayerController.SetCinematicMode` _returnvalue true true true true true))
      (:`B`
        (`KismetSystemLibrary.PrintString` "NO HELP!")
        (bind _outactors (`GameplayStatics.GetAllActorsWithTag` "MainCam"))
        (for _array_element _outactors
          (`PlayerController.SetViewTargetWithBlend` _returnvalue _array_element 1.0 "VTBlend_Linear" 0.0 false)
          (`PlayerController.SetCinematicMode` _returnvalue false true true true true))))))

(fn `UserConstructionScript`)