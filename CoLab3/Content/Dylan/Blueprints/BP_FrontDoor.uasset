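; BP_FrontDoor is the interactable front door that runs the landlord's dialogue scene once BP_Landlord has arrived.
; A trigger overlap toggles a spotlight and text prompt and enables Interact.
; Interacting blends the view to the door, hides the player in cinematic mode and opens WB_Landlord.
; Further presses advance lines and UI scenes until an empty line restores the MainCam view and player, then calls the landlord's Departure.
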(event `self.ReceiveBeginPlay`
  (`SceneComponent.SetHiddenInGame` (`self.SpotLight`) true false)
  (`SceneComponent.SetHiddenInGame` (`self.DoorText`) true false))

(event `self.trigger.OnComponentBeginOverlap`
  (params (OverlappedComponent :type "PrimitiveComponent Object Reference") (OtherActor :type "Actor Object Reference") (OtherComp :type "PrimitiveComponent Object Reference") (OtherBodyIndex :type Integer) (bFromSweep :type Boolean) (SweepResult :type "HitResult Structure (by ref)"))
  (set `self.Nearby?` true)
  (`SceneComponent.SetHiddenInGame` (`self.SpotLight`) false false)
  (`SceneComponent.SetHiddenInGame` (`self.DoorText`) false false))

(event `self.trigger.OnComponentEndOverlap`
  (params (OverlappedComponent :type "PrimitiveComponent Object Reference") (OtherActor :type "Actor Object Reference") (OtherComp :type "PrimitiveComponent Object Reference") (OtherBodyIndex :type Integer))
  (set `self.Nearby?` false)
  (`SceneComponent.SetHiddenInGame` (`self.SpotLight`) true false)
  (`SceneComponent.SetHiddenInGame` (`self.DoorText`) true false))

(event `/Game/Dylan/Blueprints/Interfaces/BPI_Interact.Interact`
  (bind _returnvalue (`GameplayStatics.GetPlayerController` 0))
  (bind _landlordui (`self.LandlordUI`))
  (if (and (`self.Nearby?`) (`self.Talking?`))
    (bind _output_get (set `self.DialogueLine` (+ (`self.DialogueLine`) 1)))
    (bind _output (`|GetArrayItem` (`self.Dialogue Text`) _output_get))
    (if (`KismetTextLibrary.TextIsEmpty` _output)
      (`KismetSystemLibrary.PrintString` "Text Over!")
      (`Widget.RemoveFromParent` (`self.LandlordUI`))
      (set `self.Talking?` false)
      (bind _outactors (`GameplayStatics.GetAllActorsWithTag` "MainCam"))
      (`PlayerController.SetViewTargetWithBlend` (`GameplayStatics.GetPlayerController` 0) (`|GetArrayItem` _outactors) 1.0 "VTBlend_Linear" 0.0 false)
      (`self.SetActorHiddenInGame` (`GameplayStatics.GetPlayerCharacter` 0) false)
      (`PlayerController.SetCinematicMode` (`GameplayStatics.GetPlayerController` 0) false true true true true)
      (set `self.Nearby?` false)
      (set `self.Talking?` false)
      (set `self.DialogueLine` 0)
      (`KismetSystemLibrary.Delay` 1.0)
      (bind _outactors_2 (`GameplayStatics.GetAllActorsWithTag` "Landlord"))
      (bind _asbp_landlord (cast `/Game/Dylan/Blueprints/BP_Landlord` (`|GetArrayItem` _outactors_2)))
      (`/Game/Dylan/Blueprints/BP_Landlord.Departure` _asbp_landlord)
      (else
        (`/Game/Dylan/UI/WB_Landlord.Update Text` _landlordui _output)
        (if (== _output_get 5)
          (`/Game/Dylan/UI/WB_Landlord.Scene1` _landlordui)
          (elif (== _output_get 1)
            (`/Game/Dylan/UI/WB_Landlord.Scene2` _landlordui)
            (elif (== _output_get 2)
              (`/Game/Dylan/UI/WB_Landlord.Scene3` _landlordui)
              (elif (== _output_get 3)
                (`/Game/Dylan/UI/WB_Landlord.Scene2` _landlordui)
                (elif (== _output_get 4)
                  (`/Game/Dylan/UI/WB_Landlord.Scene2` _landlordui))))))))
    (elif (`self.Nearby?`)
      (bind _outactors_3 (`GameplayStatics.GetAllActorsWithTag` "Landlord"))
      (bind _asbp_landlord_2 (cast `/Game/Dylan/Blueprints/BP_Landlord` (`|GetArrayItem` _outactors_3)))
      (if (`/Game/Dylan/Blueprints/BP_Landlord.Arrived?` _asbp_landlord_2)
        (`PlayerController.SetViewTargetWithBlend` _returnvalue self 1.0 "VTBlend_Linear" 0.0 false)
        (`self.SetActorHiddenInGame` (`GameplayStatics.GetPlayerCharacter` 0) true)
        (`PlayerController.SetCinematicMode` _returnvalue true true true true true)
        (`KismetSystemLibrary.PrintString` "LANDLORD?!")
        (`KismetSystemLibrary.Delay` 1.0)
        (bind _returnvalue_2 (`|CreateWidget` "/Game/Dylan/UI/WB_Landlord.WB_Landlord_C" null (`self.Speaker Name`) (`|GetArrayItem` (`self.Dialogue Text`))))
        (bind _output_get_2 (set `self.LandlordUI` _returnvalue_2))
        (`UserWidget.AddToViewport` _output_get_2 0)
        (set `self.Talking?` true)
        (else
          (`KismetSystemLibrary.PrintString` "DOOR!"))))))

(fn `UserConstructionScript`)