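; BP_Landlord is the landlord actor that walks up to a door and later leaves, hidden at BeginPlay if the game instance's Night is above zero.
; Arrival slides the Landlord component along Y with a timeline, then turns it, plays the LS_Doorshake level sequence and sets Arrived.
; Departure sets Departed, then rotates the component back while a second timeline carries it onward in the same direction.
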(event `self.ReceiveBeginPlay`
  (bind _asbp_game_instance (cast `/Game/Dylan/Blueprints/BP_GameInstance` (`GameplayStatics.GetGameInstance`)))
  (if (> (`/Game/Dylan/Blueprints/BP_GameInstance.Night` _asbp_game_instance) 0)
    (`self.SetActorHiddenInGame` true)))

(event `Arrival`
  (bind _landlord (`self.Landlord`))
  (bind (_returnvalue_x _returnvalue_y _returnvalue_z) (`KismetMathLibrary.BreakVector` (`SceneComponent.K2_GetComponentLocation` _landlord)))
  (bind _output_get (set `self.WorldPos` (`KismetMathLibrary.MakeVector` _returnvalue_x 0.0 _returnvalue_z)))
  (bind (_direction _walkin) (`Timeline|Walkin`)
    (:`Update`
      (`SceneComponent.K2_SetWorldLocation` _landlord (`KismetMathLibrary.MakeVector` (.x _output_get) (`KismetMathLibrary.Lerp` -1800.0 0.0 _walkin) (.z _output_get)) false false))
    (:`Finished`
      (`KismetSystemLibrary.MoveComponentTo` _landlord (0.0 0.0 0.0) (struct :`Yaw` -90.0) true true 1.0)
      (bind _outactor (`LevelSequencePlayer.CreateLevelSequencePlayer` "/Game/Dylan/Animations/LS_Doorshake.LS_Doorshake"))
      (`MovieSceneSequencePlayer.Play` (`LevelSequenceActor.SequencePlayer` _outactor))
      (set `self.Arrived?` true))))

(event `Departure`
  (bind _landlord (`self.Landlord`))
  (bind (_returnvalue_x _returnvalue_y _returnvalue_z) (`KismetMathLibrary.BreakVector` (`SceneComponent.K2_GetComponentLocation` _landlord)))
  (set `self.Departed?` true)
  (bind _output_get (set `self.WorldPos` (`KismetMathLibrary.MakeVector` _returnvalue_x 0.0 _returnvalue_z)))
  (`KismetSystemLibrary.MoveComponentTo` _landlord (0.0 0.0 0.0) (struct) true true 1.0)
  (bind (_direction _walkin) (`Timeline|Timeline`)
    (:`Update`
      (`SceneComponent.K2_SetWorldLocation` _landlord (`KismetMathLibrary.MakeVector` (.x _output_get) (`KismetMathLibrary.Lerp` 0.0 1800.0 _walkin) (.z _output_get)) false false))))

(fn `UserConstructionScript`)